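; Player character Blueprint that handles axis-based movement and a jump gated by a ground check.
; Move inputs add movement along the control rotation's forward and right vectors, scaled by Speed.
; Jump traces from the Cube component along its up vector by Distance, jumping only on hits tagged Ground and printing a message when nothing is hit.
; BeginPlay also runs this same trace-and-jump logic.
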(event `InputAction|Jump`
  (params (Key :type "Key Structure"))
  (bind __cube (`self. cube`))
  (bind _returnvalue (`SceneComponent.K2_GetComponentLocation` __cube))
  (:`Pressed`
    (bind (_outhit _returnvalue_2) (`KismetSystemLibrary.LineTraceSingle` :`Start` _returnvalue :`End` (+ _returnvalue (* (`KismetMathLibrary.GetUpVector` (`SceneComponent.K2_GetComponentRotation` __cube)) (`self.Distance`))) :`TraceChannel` "TraceTypeQuery1" :`DrawDebugType` "ForDuration" :!label _label))
    (if _returnvalue_2
      (if (`self.ActorHasTag` (`.HitActor` (`GameplayStatics.BreakHitResult` _outhit)) "Ground")
        (`self.Jump`))
      (else
        (`KismetSystemLibrary.PrintString` "Not on ground.")))))

(event `self.ReceiveBeginPlay`
  (goto _label))

(event `self.ReceiveTick`
  (params (DeltaSeconds :type "Float (single-precision)")))

(event `InputAxis|MoveForward`
  (params (AxisValue :type "Float (single-precision)"))
  ;[1 1 1] Move Forward
  (`self.AddMovementInput` (`KismetMathLibrary.GetForwardVector` (`self.GetControlRotation`)) (* AxisValue (`self.Speed`))))

(event `InputAxis|MoveRight`
  (params (AxisValue :type "Float (single-precision)"))
  ;[1 1 1] Move Horizontal
  (`self.AddMovementInput` (`KismetMathLibrary.GetRightVector` (`self.GetControlRotation`)) (* AxisValue (`self.Speed`))))

(fn `UserConstructionScript`)